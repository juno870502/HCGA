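; BP_RealFan is a fan actor that blows characters along its arrow direction and can be toggled by a switch.
; While on, Tick sphere-traces from the arrow and pushes the hit character with continuous force, or a single never-reset DoOnce impulse when IsOnce is set.
; ALS characters overlapping the switch flip-flop the fan's state, animation, audio and the switch's dynamic material color.
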(event OnComponentBeginOverlap(Switch)
  (params (OverlappedComponent :type Primitive%20Component%20Object%20Reference) (OtherActor :type Actor%20Object%20Reference) (OtherComp :type Primitive%20Component%20Object%20Reference) (OtherBodyIndex :type Integer) (bFromSweep :type Boolean) (SweepResult :type Hit%20Result%20Structure%20%28by%20ref%29))
  (Utilities|Casting|CastToALS_BaseCharacter_main OtherActor)
  (Utilities|FlowControl|FlipFlop
    (:A
      (Rendering|Material|SetVectorParameterValue (Variables|Default|GetSwitchMaterial) "Color" (Variables|Default|GetNewColor) :!class /Script/Engine.MaterialInstanceDynamic)
      (Variables|Default|SetOnOff false)
      (Variables|/Script/Engine.SkeletalMeshComponent|SetbPauseAnims (Variables|SkeletalMeshActor|GetSkeletalMeshComponent) true)
      (Class|AudioComponent|SetPaused (Variables|Default|GetAudio) true))
    (:B
      (Rendering|Material|SetVectorParameterValue (Variables|Default|GetSwitchMaterial) "Color" (Variables|Default|GetOrginColor) :!class /Script/Engine.MaterialInstanceDynamic)
      (Variables|Default|SetOnOff true)
      (Variables|/Script/Engine.SkeletalMeshComponent|SetbPauseAnims (Variables|SkeletalMeshActor|GetSkeletalMeshComponent) false)
      (Class|AudioComponent|SetPaused (Variables|Default|GetAudio) false))))

(event EventBeginPlay)

(event Collision|EventActorBeginOverlap
  (params (OtherActor :type Actor%20Object%20Reference)))

(event EventTick
  (params (DeltaSeconds :type Float%20%28single-precision%29))
  (bind _arrow (Variables|Default|GetArrow))
  (bind _returnvalue (Transformation|GetWorldLocation _arrow))
  (if (Variables|Default|GetOnOff)
    (bind (_outhit _returnvalue_2) (Collision|SphereTraceByChannel _returnvalue (+ _returnvalue (* (Math|Vector|GetForwardVector _arrow) (Variables|Default|GetLength))) (Variables|Default|GetRadius) "TraceTypeQuery4" false 0 "None"))
    (if _returnvalue_2
      (bind _ascharacter (Utilities|Casting|CastToCharacter (.HitActor (Collision|BreakHitResult _outhit))))
      (Variables|Default|SetOverlapCharacter _ascharacter)
      (if (Variables|Default|GetIsOnce)
        (Utilities|FlowControl|DoOnce false
          (:Completed
            (Physics|AddImpulse (Variables|/Script/Engine.Character|GetCharacterMovement (Variables|Default|GetOverlapCharacter)) (* (Math|Vector|GetForwardVector (Variables|Default|GetArrow)) (Variables|Default|GetPower)) false)))
        (else
          (Physics|AddForce (Variables|/Script/Engine.Character|GetCharacterMovement (Variables|Default|GetOverlapCharacter)) (* (Math|Vector|GetForwardVector (Variables|Default|GetArrow)) (Variables|Default|GetPower))))))))

(fn ConstructionScript
  (bind _returnvalue (Rendering|Material|CreateDynamicMaterialInstance (Variables|Default|GetSwitch) 0 "/Game/2_Material_UsedinMap/Beige_2.Beige_2" "None" :!class /Script/Engine.PrimitiveComponent))
  (bind _output_get (Variables|Default|SetSwitchMaterial _returnvalue))
  (bind _returnvalue_2 (Rendering|Material|GetVectorParameterValue _output_get "Color" :!class /Script/Engine.MaterialInstanceDynamic))
  (Variables|Default|SetOrginColor _returnvalue_2))