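; BP_PC is the player controller that manages the game's UI widgets: loading, main TimePoly screen and pause menu.
; BeginPlay shows the loading widget and records a start time, then LoadComplete swaps it for WBP_TimePoly.
; The Start input opens a reused pause widget, pausing the game with UI-only input.
; UpdateWidget fills rank slots if RankWidget exists, but its creation toggle and the achievement calls are disconnected.
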(event Custom|Load%20Complete
  (Widget|RemovefromParent (Variables|Default|GetLoadWidget))
  (bind _returnvalue (UserInterface|CreateWidget "/Game/ObjectBP/Game/UI/WBP_TimePoly.WBP_TimePoly_C"))
  (bind _output_get (Variables|Widgets|SetMainWidget _returnvalue))
  (UserInterface|Viewport|AddtoViewport _output_get 0))

(event Custom|VisiblePauseWidget
  (Utilities|IsValid (Variables|Widgets|GetPauseWidget)
    (:Is%20Valid
      _)
    (:Is%20Not%20Valid
      (bind _returnvalue (UserInterface|CreateWidget "/Game/ObjectBP/Game/UI/WBP_Pause.WBP_Pause_C"))
      (Variables|Widgets|SetPauseWidget _returnvalue)))
  (Variables|Default|SetbShowMouseCursor true)
  (Game|SetGamePaused true)
  (Input|SetInputModeUIOnly (Game|GetPlayerController 0) (Variables|Widgets|GetPauseWidget) "LockOnCapture")
  (UserInterface|Viewport|AddtoViewport (Variables|Widgets|GetPauseWidget) 0)
  (Widget|SetKeyboardFocus (Variables|Widgets|GetPauseWidget)))

(event Custom|RealStartTime)

(event EventBeginPlay
  (bind _returnvalue (UserInterface|CreateWidget "/Game/Maps/5_Loading/WBP_Loading.WBP_Loading_C"))
  (UserInterface|Viewport|AddtoViewport _returnvalue 0)
  (Variables|Default|SetLoadWidget _returnvalue)
  (Variables|Default|SetReatStartTime (Utilities|Time|GetTimeSeconds)))

(event EventUpdateWidget
  (bind _rankwidget (Variables|Default|GetRankWidget))
  ;[1 1 1] OnLeaderboardReadComplete
  (Utilities|IsValid _rankwidget
    (:Is%20Valid
      (Default|MakeRankSlot _rankwidget (Variables|Default|GetBPDataArray)))))

(event Input|ActionEvents|InputActionStart
  (params (Key :type Key%20Structure :default "None"))
  (:Pressed
    (CallFunction|VisiblePauseWidget)))

(event Input|KeyboardEvents|F
  (params (Key :type Key%20Structure :default "None")))

(event Input|KeyboardEvents|Q
  (params (Key :type Key%20Structure :default "None")))

(event Input|KeyboardEvents|E
  (params (Key :type Key%20Structure :default "None")))

(fn ConstructionScript)