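; Game mode that runs a level from loading and intro to polygon-collection ending.
; PostLogin spawns one of two characters based on the saved selection.
; BeginPlay plays loading media, streams in the room level, possesses that pawn and locks input during the intro sequence.
; Each polygon pickup updates the count and notifies the window actor; reaching the clear count writes the leaderboard and triggers the character's ending sequence.
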(event Custom|RestIgnore
  (Input|EnableInput (Game|GetPlayerCharacter 0) (Game|GetPlayerController 0))
  (Game|Player|SetViewTargetwithBlend (Game|GetPlayerController 0) (Game|Player|GetPlayerPawn 0) 1.0 "VTBlend_Cubic" 0.0 false))

(event Custom|GetPolygonGM
  (bind _windowmoved (Variables|Default|GetWindowMoved))
  (Math|Integer|IncrementInt (Variables|Default|GetCurrentPolygonNumber)
    (:%20%20
      (Utilities|FlowControl|Sequence
        (:then_0
          (Utilities|IsValid _windowmoved
            (:Is%20Valid
              (Default|CheckOpenNumber _windowmoved))))
        (:then_1
          (if (>= (Variables|Default|GetCurrentPolygonNumber) (Variables|Default|GetClearPolygonNumber))
            (CallFunction|GameEnd)))))))

(event Custom|GameEnd
  ;[1 1 1] Game End Sequence
  (bind _asbp_pc (Utilities|Casting|CastToBP_PC (Game|GetPlayerController 0)))
  (Class|MyPlayerController|WriteLeaderboard _asbp_pc)
  (bind _asals_base_character_main (Utilities|Casting|CastToALS_BaseCharacter_main (Game|Player|GetPlayerPawn 0)))
  (Default|EndingSequence _asals_base_character_main))

(event EventBeginPlay
  (bind _returnvalue (Game|GetPlayerController 0))
  (Media|MediaPlayer|OpenSource (Variables|Default|GetMP_Loading) "/Game/Maps/5_Loading/Game_Loading_ani.Game_Loading_ani")
  (Utilities|FlowControl|Delay 1.0)
  (Game|LoadStreamLevel(byName) "RoomTestLight" true)
  (bind _outactors (Actor|GetAllActorsOfClass "/Game/ObjectBP/BP_Window.BP_Window_C"))
  (Variables|Default|SetWindowMoved (Utilities|Array|Get(acopy) _outactors))
  (Pawn|Possess _returnvalue (Variables|Default|GetNewPawn))
  (bind _asbp_pc (Utilities|Casting|CastToBP_PC _returnvalue))
  (Default|LoadComplete _asbp_pc)
  (Input|DisableInput (Game|GetPlayerCharacter 0) (Game|GetPlayerController 0))
  (bind _returnvalue_2 (Sequencer|Player|CreateLevelSequencePlayer "/Game/ObjectBP/Sequence/ShotIntro.ShotIntro"))
  (Sequencer|Player|Play _returnvalue_2 :!class /Script/MovieScene.MovieSceneSequencePlayer)
  (EventDispatchers|BindEventtoOnStop _returnvalue_2 (delegate Custom|RestIgnore)))

(event EventTick
  (params (DeltaSeconds :type Float%20%28single-precision%29)))

(event EventPostLogin
  (params (NewPlayer :type Player%20Controller%20Object%20Reference))
  (bind _returnvalue (Math|Transform|MakeTransform "-4200.000000,4600.000000,1000.000000" "0.000000,180.000000,0.000000"))
  ;[1 1 1] Load Default Character
  (bind _returnvalue_2 (SaveGame|LoadGamefromSlot "BaseSlot"))
  (bind _asbp_save_game (Utilities|Casting|CastToBP_SaveGame _returnvalue_2))
  (switch int (Variables|/Game/ObjectBP/Game/BP_SaveGame.BP_SaveGame_C|GetSelectCharacter _asbp_save_game)
    (:1
      (bind _output_get (Variables|Default|SetDefaultPawnClass "/Game/DTChar/BP/BP_DTCharPA_HMK.BP_DTCharPA_HMK_C"))
      (bind _returnvalue_3 (Game|SpawnActorfromClass _output_get _returnvalue "Undefined" 0 0))
      (Variables|Default|SetNewPawn _returnvalue_3))
    (:2
      (bind _output_get_2 (Variables|Default|SetDefaultPawnClass "/Game/DTChar/BP/BP_DTCharPA_CC.BP_DTCharPA_CC_C"))
      (bind _returnvalue_4 (Game|SpawnActorfromClass _output_get_2 _returnvalue "Undefined" 0 0))
      (Variables|Default|SetNewPawn _returnvalue_4))))

(fn ConstructionScript)