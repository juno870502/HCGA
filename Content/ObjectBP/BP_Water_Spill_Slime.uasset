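; BP_Water_Spill_Slime is a slime spill object that plays squelchy step sounds while a Character is inside it.
; Two box triggers both start the sound loop on Character overlap and stop it on end overlap.
; The loop spawns SC_SlimeStep at the mesh location, repeating after random sub-second delays until a shared flag clears.
; Mesh hit and overlap events are empty, and a velocity check is left unconnected.
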(event OnComponentHit(StaticMeshComponent)
  (params (HitComponent :type Primitive%20Component%20Object%20Reference) (OtherActor :type Actor%20Object%20Reference) (OtherComp :type Primitive%20Component%20Object%20Reference) (NormalImpulse :type Vector :default "0, 0, 0") (Hit :type Hit%20Result%20Structure%20%28by%20ref%29)))

(event OnComponentBeginOverlap(StaticMeshComponent)
  (params (OverlappedComponent :type Primitive%20Component%20Object%20Reference) (OtherActor :type Actor%20Object%20Reference) (OtherComp :type Primitive%20Component%20Object%20Reference) (OtherBodyIndex :type Integer) (bFromSweep :type Boolean) (SweepResult :type Hit%20Result%20Structure%20%28by%20ref%29)))

(event OnComponentBeginOverlap(Box)
  (params (OverlappedComponent :type Primitive%20Component%20Object%20Reference) (OtherActor :type Actor%20Object%20Reference) (OtherComp :type Primitive%20Component%20Object%20Reference) (OtherBodyIndex :type Integer) (bFromSweep :type Boolean) (SweepResult :type Hit%20Result%20Structure%20%28by%20ref%29))
  (Utilities|Casting|CastToCharacter OtherActor)
  (CallFunction|PlaySoundLoop))

(event OnComponentBeginOverlap(Box1)
  (params (OverlappedComponent :type Primitive%20Component%20Object%20Reference) (OtherActor :type Actor%20Object%20Reference) (OtherComp :type Primitive%20Component%20Object%20Reference) (OtherBodyIndex :type Integer) (bFromSweep :type Boolean) (SweepResult :type Hit%20Result%20Structure%20%28by%20ref%29))
  (Utilities|Casting|CastToCharacter OtherActor)
  (CallFunction|PlaySoundLoop))

(event OnComponentEndOverlap(Box)
  (params (OverlappedComponent :type Primitive%20Component%20Object%20Reference) (OtherActor :type Actor%20Object%20Reference) (OtherComp :type Primitive%20Component%20Object%20Reference) (OtherBodyIndex :type Integer))
  (Utilities|Casting|CastToCharacter OtherActor)
  (CallFunction|EndSoundLoop))

(event OnComponentEndOverlap(Box1)
  (params (OverlappedComponent :type Primitive%20Component%20Object%20Reference) (OtherActor :type Actor%20Object%20Reference) (OtherComp :type Primitive%20Component%20Object%20Reference) (OtherBodyIndex :type Integer))
  (Utilities|Casting|CastToCharacter OtherActor)
  (CallFunction|EndSoundLoop))

(event Custom|PlaySoundLoop
  (Variables|Default|SetLoopEnable true)
  (Audio|SpawnSoundatLocation "/Game/GAME_SOUND/Effect/SlimeStep/SC_SlimeStep.SC_SlimeStep" (Transformation|GetWorldLocation (Variables|Debug|GetStaticMeshComponent)) "0, 0, 0" 1.0 1.0 0.0 0 0 :!label _label)
  (if (Variables|Default|GetLoopEnable)
    (Utilities|FlowControl|Delay (Math|Random|RandomFloat))
    (goto _label)))

(event Custom|EndSoundLoop
  (Variables|Default|SetLoopEnable false))

(event EventBeginPlay)

(event Collision|EventActorBeginOverlap
  (params (OtherActor :type Actor%20Object%20Reference)))

(event EventTick
  (params (DeltaSeconds :type Float%20%28single-precision%29)))

(fn ConstructionScript)