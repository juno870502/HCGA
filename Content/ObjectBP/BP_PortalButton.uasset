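; BP_PortalButton is a pressure-style button that switches on a portal wall when a Character steps into its trigger box.
; The construction script gives the mesh's second material slot a dynamic material instance.
; On overlap it raises that material's emissive glow and calls SwitchOnMessage on the first BP_PortalWall found in the level, with no handling to switch back off.
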(event OnComponentBeginOverlap(Box)
  (params (OverlappedComponent :type Primitive%20Component%20Object%20Reference) (OtherActor :type Actor%20Object%20Reference) (OtherComp :type Primitive%20Component%20Object%20Reference) (OtherBodyIndex :type Integer) (bFromSweep :type Boolean) (SweepResult :type Hit%20Result%20Structure%20%28by%20ref%29))
  (Utilities|Casting|CastToCharacter OtherActor)
  (Rendering|Material|SetScalarParameterValue (Variables|Default|GetMID) "Emissive_Glow_Strength" 5e+01 :!class /Script/Engine.MaterialInstanceDynamic)
  (bind _outactors (Actor|GetAllActorsOfClass "/Game/ObjectBP/BP_PortalWall.BP_PortalWall_C"))
  (Class|BPIPortal|Switchon(Message) (Utilities|Array|Get(acopy) _outactors)))

(event EventBeginPlay)

(event EventTick
  (params (DeltaSeconds :type Float%20%28single-precision%29)))

(fn ConstructionScript
  (bind _returnvalue (Rendering|Material|CreateDynamicMaterialInstance (Variables|Default|GetMI) "None" :!class /Script/Engine.KismetMaterialLibrary))
  (bind _output_get (Variables|Default|SetMID _returnvalue))
  (Rendering|Material|SetMaterial (Variables|Debug|GetStaticMeshComponent) 1 _output_get))