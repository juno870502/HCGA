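; BP_Window is a window actor that slides along Z to open once the game's polygon count reaches its threshold.
; CheckOpenNumber compares CurrentPolygonNumber from BP_GM with OpenNumber and calls OpenWindow when it is met or exceeded.
; OpenWindow plays a timeline that offsets the root's Z by TimeFlow times Length, starting from the location saved at BeginPlay.
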(event Custom|OpenWindow
  (bind _inintializevector (Variables|Default|GetInintializeVector))
  (bind (_x _y _z) (Math|Vector|BreakVector _inintializevector))
  (bind _timeflow (Timeline|타임라인_0 Play)
    (:Update
      (Transformation|SetRelativeLocation (Variables|Default|GetDefaultSceneRoot) (Math|Vector|MakeVector _x _y (+ _z (* _timeflow (Variables|Default|GetLength)))) false false))))

(event Custom|CheckOpenNumber
  (bind _asbp_gm (Utilities|Casting|CastToBP_GM (Game|GetGameMode)))
  (if (>= (Variables|/Game/ObjectBP/Game/BP_GM.BP_GM_C|GetCurrentPolygonNumber _asbp_gm) (Variables|Default|GetOpenNumber))
    (CallFunction|OpenWindow)))

(event EventBeginPlay
  (Variables|Default|SetInintializeVector (Transformation|GetActorLocation)))

(event Collision|EventActorBeginOverlap
  (params (OtherActor :type Actor%20Object%20Reference)))

(event EventTick
  (params (DeltaSeconds :type Float%20%28single-precision%29)))

(fn ConstructionScript)