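; BP_3DPrinterPlate is the moving plate of a 3D printer, toggling between an up and a down position.
; Front and inside button functions, the latter also triggered by VirtualAction, start UpPlate or DownPlate unless the plate is moving.
; Timelines lerp the actor from its current location toward the target or original location, updating the state.
; Tick reads that state to light two dynamic materials yellow while moving and dark when stopped.
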(event Custom|UpPlate
  (bind _time (Timeline|TargetTimeLine PlayFromStart)
    (:Update
      (Transformation|SetActorLocation (Math|Vector|Lerp(Vector) (Transformation|GetActorLocation) (Variables|Default|GetTargetLocation) _time) false false)
      (Variables|Default|SetState "NewEnumerator1"))
    (:Finished
      (Variables|Default|SetState "NewEnumerator2"))))

(event Custom|DownPlate
  (bind _time (Timeline|OriginalTimeLine PlayFromStart)
    (:Update
      (Transformation|SetActorLocation (Math|Vector|Lerp(Vector) (Transformation|GetActorLocation) (Variables|Default|GetOriginalLocation) _time) false false)
      (Variables|Default|SetState "NewEnumerator1"))
    (:Finished
      (Variables|Default|SetState "NewEnumerator0"))))

(event EventBeginPlay)

(event Collision|EventActorBeginOverlap
  (params (OtherActor :type Actor%20Object%20Reference)))

(event EventTick
  (params (DeltaSeconds :type Float%20%28single-precision%29))
  (switch Utilities|FlowControl|Switch|SwitchonPlateStatus (Variables|Default|GetState)
    (:NewEnumerator0
      (Rendering|Material|SetVectorParameterValue (Variables|Default|GetMI1) "EmisiveColor" "(R=0.000000,G=0.000000,B=0.000000,A=1.000000)" :!class /Script/Engine.MaterialInstanceDynamic :!label _label)
      (Rendering|Material|SetVectorParameterValue (Variables|Default|GetMI2) "EmisiveColor" "(R=0.000000,G=0.000000,B=0.000000,A=1.000000)" :!class /Script/Engine.MaterialInstanceDynamic))
    (:NewEnumerator1
      (Rendering|Material|SetVectorParameterValue (Variables|Default|GetMI1) "EmisiveColor" "(R=10.000000,G=10.000000,B=0.000000,A=1.000000)" :!class /Script/Engine.MaterialInstanceDynamic)
      (Rendering|Material|SetVectorParameterValue (Variables|Default|GetMI2) "EmisiveColor" "(R=10.000000,G=10.000000,B=0.000000,A=1.000000)" :!class /Script/Engine.MaterialInstanceDynamic))
    (:NewEnumerator2
      (goto _label))))

(event EventVirtualAction
  (params (ImpulseVector :type Vector :default "0, 0, 0"))
  (CallFunction|PushInsideButton))

(fn ConstructionScript
  (bind _returnvalue (Rendering|Material|CreateDynamicMaterialInstance (Variables|Default|GetStaticMesh4) 0 0 "None" :!class /Script/Engine.PrimitiveComponent))
  (Variables|Default|SetMI1 _returnvalue)
  (bind _returnvalue_2 (Rendering|Material|CreateDynamicMaterialInstance (Variables|Default|GetStaticMesh5) 0 0 "None" :!class /Script/Engine.PrimitiveComponent))
  (Variables|Default|SetMI2 _returnvalue_2))

(fn PushFrontButton
  (switch Utilities|FlowControl|Switch|SwitchonPlateStatus (Variables|Default|GetState)
    (:NewEnumerator0
      (CallFunction|UpPlate))
    (:NewEnumerator1
      _)
    (:NewEnumerator2
      (CallFunction|DownPlate)))
  (return true))

(fn PushInsideButton
  (switch Utilities|FlowControl|Switch|SwitchonPlateStatus (Variables|Default|GetState)
    (:NewEnumerator0
      (CallFunction|UpPlate))
    (:NewEnumerator2
      (CallFunction|DownPlate))))