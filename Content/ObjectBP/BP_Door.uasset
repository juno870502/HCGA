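; BP_Door is a door actor that swings open when a Character enters its Box trigger.
; BeginPlay caches the actor's rotation and the relative rotation of StaticMesh1, which serves as the handle.
; On overlap the DoorRot timeline plays, adding its Yaw track to the whole actor's yaw and to the handle's pitch.
; It only plays forward, with no logic to close the door.
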(event OnComponentBeginOverlap(Box)
  (params (OverlappedComponent :type Primitive%20Component%20Object%20Reference) (OtherActor :type Actor%20Object%20Reference) (OtherComp :type Primitive%20Component%20Object%20Reference) (OtherBodyIndex :type Integer) (bFromSweep :type Boolean) (SweepResult :type Hit%20Result%20Structure%20%28by%20ref%29))
  (bind _initactorrot (Variables|Default|GetInitActorRot))
  (bind _inithandlerot (Variables|Default|GetInitHandleRot))
  (bind (_roll _pitch _yaw) (Math|Rotator|BreakRotator _inithandlerot))
  (bind (_roll_2 _pitch_2 _yaw_2) (Math|Rotator|BreakRotator _initactorrot))
  (Utilities|Casting|CastToCharacter OtherActor)
  (bind _yaw_3 (Timeline|DoorRot Play)
    (:Update
      (Transformation|SetActorRotation (Math|Rotator|MakeRotator _roll_2 _pitch_2 (+ _yaw_2 _yaw_3)))
      (Transformation|SetRelativeRotation (Variables|Default|GetStaticMesh1) (Math|Rotator|MakeRotator _roll (+ _pitch _yaw_3) _yaw) false false))))

(event EventBeginPlay
  (Variables|Default|SetInitActorRot (Transformation|GetActorRotation))
  (Variables|Default|SetInitHandleRot (Variables|/Script/Engine.SceneComponent|GetRelativeRotation (Variables|Default|GetStaticMesh1))))

(event Collision|EventActorBeginOverlap
  (params (OtherActor :type Actor%20Object%20Reference)))

(event EventTick
  (params (DeltaSeconds :type Float%20%28single-precision%29)))

(fn ConstructionScript)