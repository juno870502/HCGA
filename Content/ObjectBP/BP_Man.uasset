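; BP_Man is a character object that replays a patrol animation on its skeletal mesh at a set interval.
; BeginPlay creates the looping Patrol timer and pauses it at once, and VirtualAction unpauses it.
; Start and End PawnSensing events toggle CanSeePawn, but OnSeePawn is empty and the red/green light logic reading that flag is disconnected, so it never runs.
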(event OnSeePawn(PawnSensing)
  (params (Pawn :type Pawn%20Object%20Reference)))

(event Custom|Patrol
  (Components|Animation|PlayAnimation (Variables|Default|GetSkeletalMesh) "/Game/Objects/Man/man_Anim.man_Anim" false))

(event Custom|StartPawnSensing
  (Variables|Default|SetCanSeePawn true))

(event Custom|EndPawnSensing
  (Variables|Default|SetCanSeePawn false))

(event EventBeginPlay
  (bind _returnvalue (Utilities|Time|SetTimerbyEvent (delegate Custom|Patrol) (Variables|Default|GetCycle) true))
  (bind _output_get (Variables|Default|SetTimerHandle _returnvalue))
  (Utilities|Time|PauseTimerbyHandle _output_get))

(event Collision|EventActorBeginOverlap
  (params (OtherActor :type Actor%20Object%20Reference)))

(event EventTick
  (params (DeltaSeconds :type Float%20%28single-precision%29)))

(event EventVirtualAction
  (params (ImpulseVector :type Vector :default "0, 0, 0"))
  (Utilities|Time|UnpauseTimerbyHandle (Variables|Default|GetTimerHandle)))

(fn ConstructionScript)