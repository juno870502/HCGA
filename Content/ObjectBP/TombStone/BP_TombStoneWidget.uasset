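; Tombstone actor that shows a leaderboard-backed list of tombstones on a widget component when the player reaches it.
; The first character overlap opens a quest widget, uploads today's date as a "Reach" score, requests a download and advances an achievement.
; A timer then passes BPTombArray to the list widget and fades it in with a timeline.
; End overlap still calls a test-only achievement reset marked for removal before release.
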(event OnComponentBeginOverlap(Box)
  (params (OverlappedComponent :type Primitive%20Component%20Object%20Reference) (OtherActor :type Actor%20Object%20Reference) (OtherComp :type Primitive%20Component%20Object%20Reference) (OtherBodyIndex :type Integer) (bFromSweep :type Boolean) (SweepResult :type Hit%20Result%20Structure%20%28by%20ref%29))
  (bind _returnvalue (Game|GetPlayerController 0))
  (Utilities|FlowControl|DoOnce false
    (:Completed
      (Utilities|Casting|CastToALS_BaseCharacter_main OtherActor)
      (bind _returnvalue_2 (UserInterface|CreateWidget "/Game/ObjectBP/Game/UI/WBP_TombstoneQuest.WBP_TombstoneQuest_C"))
      (UserInterface|Viewport|AddtoViewport _returnvalue_2 0)
      (CallFunction|WriteTombstone)
      (Utilities|FlowControl|Delay 0.5)
      (CallFunction|ReadTombstone)
      (Utilities|Time|SetTimerbyEvent (delegate Custom|DrawEvent) 1.0)
      ;[1 1 1] Tombstone Achievement
      (|CacheAchievements _returnvalue
        (:OnSuccess
          (|WriteAchievementProgress _returnvalue "ACH_G_A" 1e+02
            (:then
              (Development|PrintString "Tomb Progress"))))))))

(event OnComponentEndOverlap(Box)
  (params (OverlappedComponent :type Primitive%20Component%20Object%20Reference) (OtherActor :type Actor%20Object%20Reference) (OtherComp :type Primitive%20Component%20Object%20Reference) (OtherBodyIndex :type Integer))
  ;[1 0 0] OnlyTest! Delete In Release!
  (Development|PrintString "Reset!")
  (Class|MyActorTombstone|TestOnlyResetAhievements))

(event Custom|DrawEvent
  (CallFunction|BeginDrawTombstone (Variables|Default|GetBPTombArray)))

(event Custom|BeginDrawTombstone
  (params (TombArray :type Array%20of%20Tomb%20Stone%20Leaderboard%20Structures))
  (bind _aswbp_tomb_stone_list (Utilities|Casting|CastToWBP_TombStoneList (UserInterface|GetUserWidgetObject (Variables|Default|GetWidget))))
  (Utilities|IsValid _aswbp_tomb_stone_list
    (:Is%20Valid
      (Default|MakeTombstone _aswbp_tomb_stone_list TombArray)
      (bind _opacity (Timeline|DrawTombstone Play)
        (:Update
          (Class|WidgetComponent|SetTintColorandOpacity (Variables|Default|GetWidget) (Utilities|Struct|MakeLinearColor 1.0 1.0 1.0 _opacity)))))))

(event Custom|WriteTombstone
  (Class|MyActorTombstone|FindLeaderboard "Reach")
  (Variables|Default|SetIsWrite true))

(event Custom|ReadTombstone
  (Class|MyActorTombstone|FindLeaderboard "Reach")
  (Variables|Default|SetIsWrite false))

(event EventBeginPlay)

(event EventTick
  (params (DeltaSeconds :type Float%20%28single-precision%29)))

(event Collision|EventActorBeginOverlap
  (params (OtherActor :type Actor%20Object%20Reference)))

(event EventOnFindLeaderboardEvent
  (bind _returnvalue (Math|DateTime|Now))
  (bind (_year _month _day) (Math|DateTime|BreakDateTime _returnvalue))
  (if (Variables|Default|GetIsWrite)
    (Class|MyActorTombstone|UploadScore (+ (* _year 10000) (* _month 100) _day 0))
    (else
      (Class|MyActorTombstone|DownloadScores))))

(fn ConstructionScript)