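; BP_VolumeWorldEnd is a trigger volume that records and displays tombstones when a character enters its box.
; On overlap, it has the first player controller (BP_PC) write, then read tombstone data, regardless of which character entered.
; A one-second timer then passes the controller's tombstone array to the first BP_TombStoneWidget actor, found at BeginPlay, to begin drawing.
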(event OnComponentBeginOverlap(Box)
  (params (OverlappedComponent :type Primitive%20Component%20Object%20Reference) (OtherActor :type Actor%20Object%20Reference) (OtherComp :type Primitive%20Component%20Object%20Reference) (OtherBodyIndex :type Integer) (bFromSweep :type Boolean) (SweepResult :type Hit%20Result%20Structure%20%28by%20ref%29))
  (Utilities|Casting|CastToCharacter OtherActor)
  (bind _asbp_pc (Utilities|Casting|CastToBP_PC (Game|GetPlayerController 0)))
  (Default|WriteTombstone _asbp_pc)
  (Default|ReadTombstone _asbp_pc)
  (Utilities|Time|SetTimerbyEvent (delegate Custom|DrawEvent) 1.0))

(event Custom|DrawEvent
  (Default|BeginDrawTombstone (Variables|Default|GetTombstoneWidget) (Variables|/Script/HCGA.MyPlayerController|GetBPTombArray (stale OnComponentBeginOverlap(Box) _asbp_pc))))

(event EventBeginPlay
  (bind _outactors (Actor|GetAllActorsOfClass "/Game/ObjectBP/TombStone/BP_TombStoneWidget.BP_TombStoneWidget_C"))
  (Variables|Default|SetTombstoneWidget (Utilities|Array|Get(acopy) _outactors)))

(event Collision|EventActorBeginOverlap
  (params (OtherActor :type Actor%20Object%20Reference)))

(event EventTick
  (params (DeltaSeconds :type Float%20%28single-precision%29)))

(fn ConstructionScript)