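; BP_Warp is a linked warp point that teleports an overlapping Character to the location of its OutWarp.
; A use counter gates it, with negative values acting as unlimited, and drops on each accepted overlap, even when teleporting is disabled.
; Teleporting disables OutWarp until an overlap ends there, preventing bounce-back, then zeroes velocity and plays a DoOnce-gated sound.
; The construction script tints the particle system with a brightened Color.
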(event EventBeginPlay)

(event Collision|EventActorBeginOverlap
  (params (OtherActor :type Actor%20Object%20Reference))
  (if (or (< (Variables|Default|GetNumOfAvailable) 0) (> (Variables|Default|GetNumOfAvailable) 0))
    (Math|Integer|DecrementInt (Variables|Default|GetNumOfAvailable)
      (:%20%20
        (if (Variables|Default|GetCanTeleport)
          (Variables|BP_Warp_C|SetCanTeleport (Variables|Default|GetOutWarp) false)
          (bind _ascharacter (Utilities|Casting|CastToCharacter OtherActor))
          (Variables|/Script/Engine.MovementComponent|SetVelocity (Pawn|GetMovementComponent _ascharacter) "0, 0, 0")
          (Transformation|SetActorLocation OtherActor (Transformation|GetActorLocation (Variables|Default|GetOutWarp)) false false)
          (Utilities|FlowControl|DoOnce false
            (:Completed
              (Audio|PlaySoundatLocation "/Game/GAME_SOUND/SC_Warp.SC_Warp" (Transformation|GetActorLocation) "0, 0, 0" 1.0 1.0 0.0 0 0 0))))))))

(event EventTick
  (params (DeltaSeconds :type Float%20%28single-precision%29)))

(event Collision|EventActorEndOverlap
  (params (OtherActor :type Actor%20Object%20Reference))
  (if (not (Variables|Default|GetCanTeleport))
    (Variables|Default|SetCanTeleport true)
    (Utilities|FlowControl|DoOnce false) ; enters at Reset
  ))

(fn ConstructionScript
  (bind _color (Variables|Default|GetColor))
  (bind (_b _g _r) (Math|Color|BreakColor _color))
  (Effects|Components|ParticleSystem|SetVectorParameter (Variables|Default|GetParticleSystem) "Color" (* (Math|Vector|MakeVector (Math|Conversions|ToFloat(Byte) _r) (Math|Conversions|ToFloat(Byte) _g) (Math|Conversions|ToFloat(Byte) _b)) 10)))