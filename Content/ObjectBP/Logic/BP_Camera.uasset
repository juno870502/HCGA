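; BP_Camera is an actor that keeps turning to face the game's character, acting as a look-at camera judging by its name.
; On BeginPlay it caches the first Character actor found in the level.
; Every Tick, while that reference is valid, it sets its own rotation to the look-at rotation from its location to the character's, snapping without interpolation.
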(event EventBeginPlay
  (bind _outactors (Actor|GetAllActorsOfClass "/Script/Engine.Character"))
  (Variables|Default|SetCharacter (Utilities|Array|Get(acopy) _outactors)))

(event Collision|EventActorBeginOverlap
  (params (OtherActor :type Actor%20Object%20Reference)))

(event EventTick
  (params (DeltaSeconds :type Float%20%28single-precision%29))
  (Utilities|IsValid (Variables|Default|GetCharacter)
    (:Is%20Valid
      (Transformation|SetActorRotation (Math|Rotator|FindLookatRotation (Transformation|GetActorLocation) (Transformation|GetActorLocation (Variables|Default|GetCharacter)))))))

(fn ConstructionScript)