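; BP_CC_BGM is a background music volume that fades music in and out as a Character enters and leaves its box.
; BeginPlay assigns the Sound variable to the audio component, and box overlaps drive the fades.
; When Intro is set, each entry starts a timer lasting the sound's duration, then swaps to a hardcoded Chochoroomtheme2 cue.
; Exiting does not clear that timer.
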(event OnComponentBeginOverlap(Box)
  (params (OverlappedComponent :type Primitive%20Component%20Object%20Reference) (OtherActor :type Actor%20Object%20Reference) (OtherComp :type Primitive%20Component%20Object%20Reference) (OtherBodyIndex :type Integer) (bFromSweep :type Boolean) (SweepResult :type Hit%20Result%20Structure%20%28by%20ref%29))
  (Utilities|Casting|CastToCharacter OtherActor)
  (Audio|Components|Audio|FadeIn (Variables|Default|GetAudio1) (Variables|Default|GetFadeInDuration) 1.0 0.0 "Linear" :!class /Script/Engine.AudioComponent)
  (if (Variables|Default|GetIntro)
    (Utilities|Time|SetTimerbyEvent (delegate Custom|SetSecondSound) (Variables|/Script/Engine.SoundBase|GetDuration (Variables|Default|GetSound)))))

(event OnComponentEndOverlap(Box)
  (params (OverlappedComponent :type Primitive%20Component%20Object%20Reference) (OtherActor :type Actor%20Object%20Reference) (OtherComp :type Primitive%20Component%20Object%20Reference) (OtherBodyIndex :type Integer))
  (Utilities|Casting|CastToCharacter OtherActor)
  (Audio|Components|Audio|FadeOut (Variables|Default|GetAudio1) 2.0 0.0 "Linear" :!class /Script/Engine.AudioComponent))

(event Custom|SetSecondSound
  (Audio|Components|Audio|SetSound (Variables|Default|GetAudio1) "/Game/GAME_SOUND/Music/Loop/chochoroomtheme2_Cue.chochoroomtheme2_Cue"))

(event EventBeginPlay
  (Audio|Components|Audio|SetSound (Variables|Default|GetAudio1) (Variables|Default|GetSound)))

(event Collision|EventActorBeginOverlap
  (params (OtherActor :type Actor%20Object%20Reference)))

(event EventTick
  (params (DeltaSeconds :type Float%20%28single-precision%29)))

(fn ConstructionScript)