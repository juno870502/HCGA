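; BP_VolumeBGMOnOff is a box trigger volume that fades a background music sound in and out for the player character class.
; BeginPlay assigns the configured Sound to the Audio component, and only overlaps by ALS_BaseCharacter_main count.
; With IsFlipflop set, each entry alternates between fade in and fade out, and exits are ignored.
; Otherwise, the music fades in on entry and out on exit.
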(event OnComponentBeginOverlap(Box)
  (params (OverlappedComponent :type Primitive%20Component%20Object%20Reference) (OtherActor :type Actor%20Object%20Reference) (OtherComp :type Primitive%20Component%20Object%20Reference) (OtherBodyIndex :type Integer) (bFromSweep :type Boolean) (SweepResult :type Hit%20Result%20Structure%20%28by%20ref%29))
  (bind _audio (Variables|Default|GetAudio))
  (Utilities|Casting|CastToALS_BaseCharacter_main OtherActor)
  (if (Variables|Default|GetIsFlipflop)
    (Utilities|FlowControl|FlipFlop
      (:A
        (Audio|Components|Audio|FadeIn _audio 1.0 1.0 0.0 "Linear" :!class /Script/Engine.AudioComponent))
      (:B
        (Audio|Components|Audio|FadeOut _audio 1.0 0.0 "Linear" :!class /Script/Engine.AudioComponent)))
    (else
      (Audio|Components|Audio|FadeIn (Variables|Default|GetAudio) 1.0 1.0 0.0 "Linear" :!class /Script/Engine.AudioComponent))))

(event OnComponentEndOverlap(Box)
  (params (OverlappedComponent :type Primitive%20Component%20Object%20Reference) (OtherActor :type Actor%20Object%20Reference) (OtherComp :type Primitive%20Component%20Object%20Reference) (OtherBodyIndex :type Integer))
  (Utilities|Casting|CastToALS_BaseCharacter_main OtherActor)
  (if (not (Variables|Default|GetIsFlipflop))
    (Audio|Components|Audio|FadeOut (Variables|Default|GetAudio) 1.0 0.0 "Linear" :!class /Script/Engine.AudioComponent)))

(event EventBeginPlay
  (Audio|Components|Audio|SetSound (Variables|Default|GetAudio) (Variables|Default|GetSound)))

(event Collision|EventActorBeginOverlap
  (params (OtherActor :type Actor%20Object%20Reference)))

(event EventTick
  (params (DeltaSeconds :type Float%20%28single-precision%29)))

(fn ConstructionScript)