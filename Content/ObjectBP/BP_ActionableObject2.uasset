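; BP_ActionableObject2 is a physics prop that can be pushed by an action and makes a sound on hard impacts.
; VirtualAction applies the incoming vector, scaled by ImpulsePower, as an impulse to the static mesh.
; On component hit, it spawns SC_Mic at the actor's location if mesh speed exceeds a threshold.
; The construction script assigns a configurable mesh and a dynamic material with a random Base color.
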(event OnComponentHit(StaticMesh)
  (params (HitComponent :type Primitive%20Component%20Object%20Reference) (OtherActor :type Actor%20Object%20Reference) (OtherComp :type Primitive%20Component%20Object%20Reference) (NormalImpulse :type Vector :default "0, 0, 0") (Hit :type Hit%20Result%20Structure%20%28by%20ref%29))
  (bind _returnvalue (Physics|GetPhysicsLinearVelocity (Variables|Default|GetStaticMesh) "None"))
  (if (> (Math|Vector|VectorLength _returnvalue) 3e+02)
    (Audio|SpawnSoundatLocation "/Game/GAME_SOUND/Item/Mic/SC_Mic.SC_Mic" (Transformation|GetActorLocation) "0, 0, 0" 1.0 1.0 0.0 0 0)))

(event EventBeginPlay)

(event Collision|EventActorBeginOverlap
  (params (OtherActor :type Actor%20Object%20Reference)))

(event EventTick
  (params (DeltaSeconds :type Float%20%28single-precision%29)))

(event EventVirtualAction
  (params (ImpulseVector :type Vector :default "0, 0, 0"))
  (Physics|AddImpulse (Variables|Default|GetStaticMesh) (* ImpulseVector (Variables|Default|GetImpulsePower)) "None" false))

(fn ConstructionScript
  (bind _returnvalue (Math|Random|RandomUnitVector))
  (bind _staticmesh (Variables|Default|GetStaticMesh))
  (Components|StaticMesh|SetStaticMesh _staticmesh (Variables|Default|GetNewMesh))
  (bind _returnvalue_2 (Rendering|Material|CreateDynamicMaterialInstance _staticmesh 0 (Variables|Default|GetMI) "None" :!class /Script/Engine.PrimitiveComponent))
  (Rendering|Material|SetVectorParameterValue _returnvalue_2 "Base" (Utilities|Struct|MakeLinearColor (.x _returnvalue) (.y _returnvalue) (.z _returnvalue) 1.0) :!class /Script/Engine.MaterialInstanceDynamic))