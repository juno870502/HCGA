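; BP_Jar is a physics jar prop that shakes and then gets knocked sideways when its VirtualAction event fires.
; VirtualAction starts a looping timer that repeatedly pops the static mesh upward, plus a one-shot timer for the fall.
; After a few seconds FallingEvent shoves the mesh along negative Y and clears both timers.
; Both impulses apply as velocity changes, so the motion ignores mass.
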(event Custom|FallingEvent
  (Physics|AddImpulse (Variables|Default|GetStaticMesh) "0,-700.000000,0.000000" "None" true)
  (Utilities|Time|ClearandInvalidateTimerbyHandle (Variables|Default|GetShakingTimerHandle))
  (Utilities|Time|ClearandInvalidateTimerbyHandle (stale EventVirtualAction _returnvalue_2)))

(event Custom|ShakingEvent
  (Physics|AddImpulse (Variables|Default|GetStaticMesh) "0,0.000000,100.000000" "None" true))

(event EventBeginPlay)

(event Collision|EventActorBeginOverlap
  (params (OtherActor :type Actor%20Object%20Reference)))

(event EventTick
  (params (DeltaSeconds :type Float%20%28single-precision%29)))

(event EventVirtualAction
  (params (ImpulseVector :type Vector :default "0, 0, 0"))
  (bind _returnvalue (Utilities|Time|SetTimerbyEvent (delegate Custom|ShakingEvent) 0.3 true))
  (Variables|Default|SetShakingTimerHandle _returnvalue)
  (bind _returnvalue_2 (Utilities|Time|SetTimerbyEvent (delegate Custom|FallingEvent) 5.0)))

(fn ConstructionScript)