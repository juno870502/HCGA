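; BP_Speaker is an interactive speaker that plays audio and notifies a Ted bear actor (Ted2_Blueprint).
; BeginPlay caches the first bear in the level; VirtualAction starts the audio, messages the bear and sets IsPlaying.
; When the audio finishes, it messages the bear again and clears the flag.
; A Character leaving the Box during playback fades the audio out; the begin-overlap branch is empty.
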(event OnAudioFinished(Audio)
  (Class|BPIAction|VirtualAction(Message) (Variables|Default|GetTedBear) "0, 0, 0")
  (Variables|Default|SetIsPlaying false))

(event OnComponentBeginOverlap(Box)
  (params (OverlappedComponent :type Primitive%20Component%20Object%20Reference) (OtherActor :type Actor%20Object%20Reference) (OtherComp :type Primitive%20Component%20Object%20Reference) (OtherBodyIndex :type Integer) (bFromSweep :type Boolean) (SweepResult :type Hit%20Result%20Structure%20%28by%20ref%29))
  (Utilities|Casting|CastToCharacter OtherActor)
  (if (Variables|Default|GetIsPlaying)
    _))

(event OnComponentEndOverlap(Box)
  (params (OverlappedComponent :type Primitive%20Component%20Object%20Reference) (OtherActor :type Actor%20Object%20Reference) (OtherComp :type Primitive%20Component%20Object%20Reference) (OtherBodyIndex :type Integer))
  (Utilities|Casting|CastToCharacter OtherActor)
  (if (Variables|Default|GetIsPlaying)
    (Audio|Components|Audio|FadeOut (Variables|Default|GetAudio) 1.0 0.0 "Linear" :!class /Script/Engine.AudioComponent)))

(event EventBeginPlay
  (bind _outactors (Actor|GetAllActorsOfClass "/Game/ObjectBP/Speaker/Ted2_Blueprint.Ted2_Blueprint_C"))
  (Variables|Default|SetTedBear (Utilities|Array|Get(acopy) _outactors)))

(event Collision|EventActorBeginOverlap
  (params (OtherActor :type Actor%20Object%20Reference)))

(event EventTick
  (params (DeltaSeconds :type Float%20%28single-precision%29)))

(event EventVirtualAction
  (params (ImpulseVector :type Vector :default "0, 0, 0"))
  (bind _tedbear (Variables|Default|GetTedBear))
  (Components|Activation|Activate (Variables|Default|GetAudio) false)
  (Utilities|IsValid _tedbear
    (:Is%20Valid
      (Class|BPIAction|VirtualAction(Message) _tedbear "0, 0, 0")
      (Variables|Default|SetIsPlaying true))))

(fn ConstructionScript)