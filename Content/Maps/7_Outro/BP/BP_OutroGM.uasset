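; BP_OutroGM is the game mode for the Outro map, which plays the ending movie and then moves on to the Rank level.
; BeginPlay opens OutroMovie on the MPOutro media player, and its end-reached event fires OpenLevelTimer to load Rank.
; A disconnected demo variant would loop a farewell clip with an audio fade-in, and a separate PlayMPTexture event restarts playback.
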(event Custom|OpenLevelTimerDemo
  ;[1 1 1] Outro - Demoversion
  (Game|OpenLevel(byName) "Rank"))

(event Custom|OpenLevelTimer
  ;[1 1 1] Outro - In Demo Not Play
  (Game|OpenLevel(byName) "Rank"))

(event Custom|Play%20MP%20Texture
  (Media|MediaPlayer|Play (Variables|Default|GetMP_Outro) :!class /Script/MediaAssets.MediaPlayer))

(event EventBeginPlay
  (bind _mp_outro (Variables|Default|GetMP_Outro))
  ;[1 1 1] Outro - In Demo Not Play
  (Media|MediaPlayer|OpenSource _mp_outro "/Game/Maps/7_Outro/OutroMovie.OutroMovie")
  (Media|MediaPlayer|Play _mp_outro :!class /Script/MediaAssets.MediaPlayer)
  (Media|MediaPlayer|BindEventtoOnEndReached _mp_outro (delegate Custom|OpenLevelTimer)))

(event EventTick
  (params (DeltaSeconds :type Float%20%28single-precision%29)))

(fn ConstructionScript)