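; Player controller for the character select screen, which creates the selection widget and lets the player pick one of two characters (HMK or CC).
; The MoveRight/Left axis highlights a character on the widget and records the choice.
; Any of four action inputs confirms once, locking input through IsPlayed, playing audio and async-saving the choice to a new BP_SaveGame.
; When the audio finishes, it opens the RoomTestLight level.
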(event Custom|OnAudioFinished_Event_0
  (Game|OpenLevel(byName) "RoomTestLight"))

(event EventBeginPlay
  (bind _returnvalue (UserInterface|CreateWidget "/Game/Maps/Select/BluePrint/BPSelectWidget.BPSelectWidget_C"))
  (bind _output_get (Variables|Default|SetSelectWidget _returnvalue))
  (UserInterface|Viewport|AddtoViewport _output_get 0))

(event EventTick
  (params (DeltaSeconds :type Float%20%28single-precision%29)))

(event Input|ActionEvents|InputActionRagdollAction
  (params (Key :type Key%20Structure :default "None"))
  (bind _audio (Variables|Default|GetAudio))
  (:Pressed
    (if (Variables|Default|GetIsCharSelect)
      (if (Variables|Default|GetIsPlayed)
        (Variables|Default|SetIsPlayed false)
        (Audio|Components|Audio|Play _audio 0.0)
        (EventDispatchers|BindEventtoOnAudioFinished _audio (delegate Custom|OnAudioFinished_Event_0))
        (bind _returnvalue (SaveGame|CreateSaveGameObject "/Game/ObjectBP/Game/BP_SaveGame.BP_SaveGame_C"))
        (Variables|/Game/ObjectBP/Game/BP_SaveGame.BP_SaveGame_C|SetSelectCharacter _returnvalue (Variables|Default|GetSelectCharacterPC))
        (|AsyncSaveGametoSlot _returnvalue (Variables|/Game/ObjectBP/Game/BP_SaveGame.BP_SaveGame_C|GetSaveSlotName _returnvalue) (Variables|/Game/ObjectBP/Game/BP_SaveGame.BP_SaveGame_C|GetUserIndex _returnvalue))))))

(event Input|ActionEvents|InputActionAction
  (params (Key :type Key%20Structure :default "None"))
  (bind _audio (Variables|Default|GetAudio))
  (:Pressed
    (if (Variables|Default|GetIsCharSelect)
      (if (Variables|Default|GetIsPlayed)
        (Variables|Default|SetIsPlayed false)
        (Audio|Components|Audio|Play _audio 0.0)
        (EventDispatchers|BindEventtoOnAudioFinished _audio (delegate Custom|OnAudioFinished_Event_0))
        (bind _returnvalue (SaveGame|CreateSaveGameObject "/Game/ObjectBP/Game/BP_SaveGame.BP_SaveGame_C"))
        (Variables|/Game/ObjectBP/Game/BP_SaveGame.BP_SaveGame_C|SetSelectCharacter _returnvalue (Variables|Default|GetSelectCharacterPC))
        (|AsyncSaveGametoSlot _returnvalue (Variables|/Game/ObjectBP/Game/BP_SaveGame.BP_SaveGame_C|GetSaveSlotName _returnvalue) (Variables|/Game/ObjectBP/Game/BP_SaveGame.BP_SaveGame_C|GetUserIndex _returnvalue))))))

(event Input|ActionEvents|InputActionJumpAction
  (params (Key :type Key%20Structure :default "None"))
  (bind _audio (Variables|Default|GetAudio))
  (:Pressed
    (if (Variables|Default|GetIsCharSelect)
      (if (Variables|Default|GetIsPlayed)
        (Variables|Default|SetIsPlayed false)
        (Audio|Components|Audio|Play _audio 0.0)
        (EventDispatchers|BindEventtoOnAudioFinished _audio (delegate Custom|OnAudioFinished_Event_0))
        (bind _returnvalue (SaveGame|CreateSaveGameObject "/Game/ObjectBP/Game/BP_SaveGame.BP_SaveGame_C"))
        (Variables|/Game/ObjectBP/Game/BP_SaveGame.BP_SaveGame_C|SetSelectCharacter _returnvalue (Variables|Default|GetSelectCharacterPC))
        (|AsyncSaveGametoSlot _returnvalue (Variables|/Game/ObjectBP/Game/BP_SaveGame.BP_SaveGame_C|GetSaveSlotName _returnvalue) (Variables|/Game/ObjectBP/Game/BP_SaveGame.BP_SaveGame_C|GetUserIndex _returnvalue))))))

(event Input|ActionEvents|InputActionStanceAction
  (params (Key :type Key%20Structure :default "None"))
  (bind _audio (Variables|Default|GetAudio))
  (:Pressed
    (if (Variables|Default|GetIsCharSelect)
      (if (Variables|Default|GetIsPlayed)
        (Variables|Default|SetIsPlayed false)
        (Audio|Components|Audio|Play _audio 0.0)
        (EventDispatchers|BindEventtoOnAudioFinished _audio (delegate Custom|OnAudioFinished_Event_0))
        (bind _returnvalue (SaveGame|CreateSaveGameObject "/Game/ObjectBP/Game/BP_SaveGame.BP_SaveGame_C"))
        (Variables|/Game/ObjectBP/Game/BP_SaveGame.BP_SaveGame_C|SetSelectCharacter _returnvalue (Variables|Default|GetSelectCharacterPC))
        (|AsyncSaveGametoSlot _returnvalue (Variables|/Game/ObjectBP/Game/BP_SaveGame.BP_SaveGame_C|GetSaveSlotName _returnvalue) (Variables|/Game/ObjectBP/Game/BP_SaveGame.BP_SaveGame_C|GetUserIndex _returnvalue))))))

(event Input|AxisEvents|InputAxisMoveRight/Left
  (params (AxisValue :type Float%20%28single-precision%29))
  (if (not (== AxisValue 0.0))
    (if (Variables|Default|GetIsPlayed)
      (if (< AxisValue 0.0)
        (Default|HMKSeleted (Variables|Default|GetSelectWidget))
        (Variables|Default|SetIsCharSelect true)
        (Variables|Default|SetIsHMK true)
        (Variables|Default|SetSelectCharacterPC 1)
        (else
          (Default|CCSelected (Variables|Default|GetSelectWidget))
          (Variables|Default|SetIsCharSelect true)
          (Variables|Default|SetIsHMK false)
          (Variables|Default|SetSelectCharacterPC 2))))))

(fn ConstructionScript)