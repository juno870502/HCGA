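; BP_MMPC is the main menu player controller that puts up the menu and rank UI.
; On BeginPlay it creates BP_MMWidget, shows the mouse cursor and sets Game and UI input focused on that widget.
; CreateRankWidget spawns and stores a WBP_Rank widget, which UpdateWidget fills through MakeRankSlot using BPDataArray when the widget is valid.
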(event Custom|Create%20Rank%20Widget
  (bind _returnvalue (UserInterface|CreateWidget "/Game/ObjectBP/Game/UI/WBP_Rank.WBP_Rank_C"))
  (UserInterface|Viewport|AddtoViewport _returnvalue 0)
  (Variables|Default|SetRankWidget _returnvalue))

(event EventBeginPlay
  (bind _returnvalue (UserInterface|CreateWidget "/Game/Maps/3_MainMenu/BP_MMWidget.BP_MMWidget_C"))
  (UserInterface|Viewport|AddtoViewport _returnvalue 0)
  (Variables|Default|SetbShowMouseCursor true)
  (Input|SetInputModeGameandUI self _returnvalue "DoNotLock" true))

(event EventTick
  (params (DeltaSeconds :type Float%20%28single-precision%29)))

(event EventUpdateWidget
  (bind _rankwidget (Variables|Default|GetRankWidget))
  (Utilities|IsValid _rankwidget
    (:Is%20Valid
      (Default|MakeRankSlot _rankwidget (Variables|Default|GetBPDataArray)))))

(fn ConstructionScript)