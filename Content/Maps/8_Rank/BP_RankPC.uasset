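; Player controller for the rank map that shows the player's time result in a UI-only personal rank widget, currently wired as the demo version.
; BeginPlay starts a "Time" leaderboard lookup, creates the personal rank and end-link widgets, and fills the time from ProjectGameInstance.
; The find callback downloads personal scores, but main-version global widget creation and personal rank display are disconnected, leaving UpdateWidget effectively inactive.
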(event Custom|Demo%20Rank
  (bind _asproject_game_instance (Utilities|Casting|CastToProjectGameInstance (Game|GetGameInstance)))
  (Default|MakeTimeScoreDemo (Variables|Default|GetPersonalRankWidget) (Variables|/Script/HCGA.ProjectGameInstance|GetGameTimeScore _asproject_game_instance)))

(event Custom|CreateRankWidgets
  (bind _returnvalue (UserInterface|CreateWidget "/Game/ObjectBP/Game/UI/WBP_PersonalRank.WBP_PersonalRank_C"))
  (Variables|Default|SetPersonalRankWidget _returnvalue)
  ;[1 1 1] Demo Version
  (bind _returnvalue_2 (UserInterface|CreateWidget "/Game/ObjectBP/Game/UI/WBP_EndLink.WBP_EndLink_C"))
  (Variables|Default|SetEndLink _returnvalue_2)
  (CallFunction|DemoRank))

(event EventBeginPlay
  (bind _personalrankwidget (Variables|Default|GetPersonalRankWidget))
  (Class|MyPlayerController|FindLeaderboard "Time")
  (CallFunction|CreateRankWidgets)
  (UserInterface|Viewport|AddtoViewport _personalrankwidget 0)
  (Input|SetInputModeUIOnly self _personalrankwidget "DoNotLock")
  (Variables|Default|SetbShowMouseCursor true))

(event EventTick
  (params (DeltaSeconds :type Float%20%28single-precision%29)))

(event EventOnFindLeaderboardEvent
  (Class|MyPlayerController|DownloadScores "Personal"))

(event EventOnDownloadLeaderboardEvent)

(event EventUpdateWidget
  (bind _globalrankwidget (Variables|Default|GetGlobalRankWidget))
  (if (< (Utilities|Array|Length (Variables|Default|GetBPDataArray)) 2)
    (Utilities|IsValid (Variables|Default|GetPersonalRankWidget))
    (else
      (Utilities|IsValid _globalrankwidget
        (:Is%20Valid
          (Default|MakeRankSlot _globalrankwidget (Variables|Default|GetBPDataArray)))))))

(fn ConstructionScript)